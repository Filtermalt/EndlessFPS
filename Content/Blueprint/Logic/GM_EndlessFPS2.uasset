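; Game mode for an endless FPS level that manages a chain of BP_Spawner actors and their sequential tile destruction.
; BeginPlay spawns three spawners at NextSpawnPoint into SpawnerArray and starts tile destruction on the first.
; AddSpawner appends another at NextSpawnPoint, which this graph reads but never updates.
; A looping timer polls the current spawner and, once it is invalid, advances Index to start destruction on the next.
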(event EventBeginPlay
  (bind _returnvalue (Game|SpawnActorfromClass "/Game/Blueprint/Floor/BP_Spawner.BP_Spawner_C" (Variables|Default|GetNextSpawnPoint) "Undefined" 0 0))
  (Default|StartDestroyTiles _returnvalue)
  (Utilities|Array|Add (Variables|Default|GetSpawnerArray) _returnvalue)
  (for _index (range 0 1)
    (bind _returnvalue_2 (Game|SpawnActorfromClass "/Game/Blueprint/Floor/BP_Spawner.BP_Spawner_C" (Variables|Default|GetNextSpawnPoint) "Undefined" 0 0))
    (Utilities|Array|Add (Variables|Default|GetSpawnerArray) _returnvalue_2))
  (Utilities|Time|SetTimerbyFunctionName 0 "DestroyTilesCheck" 0.5 true))

(fn ConstructionScript)

(fn AddSpawner
  (bind _returnvalue (Game|SpawnActorfromClass "/Game/Blueprint/Floor/BP_Spawner.BP_Spawner_C" (Variables|Default|GetNextSpawnPoint) "Undefined" 0 0))
  (Utilities|Array|Add (Variables|Default|GetSpawnerArray) _returnvalue))

(fn DestroyTilesCheck
  (Utilities|IsValid (Utilities|Array|Get(acopy) (Variables|Default|GetSpawnerArray) (Variables|Default|Getindex))
    (:Is%20Not%20Valid
      (Variables|Default|Setindex (+ (Variables|Default|Getindex) 1))
      (Default|StartDestroyTiles (Utilities|Array|Get(acopy) (Variables|Default|GetSpawnerArray) (Variables|Default|Getindex))))))