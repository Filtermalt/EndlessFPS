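; Floor tile Blueprint for a left/right fork in the endless FPS mode, registering which branch the player takes.
; LeftBox and RightBox overlaps react only to FirstPersonCharacter, setting a left or right Direction on GM_EndlessFPS2 and clearing its IsTwoRoads flag.
; A disconnected node that would copy the game mode's SecondSpawnPoint into NextSpawnPoint never runs.
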(event OnComponentBeginOverlap(LeftBox)
  (params (OverlappedComponent :type Primitive%20Component%20Object%20Reference) (OtherActor :type Actor%20Object%20Reference) (OtherComp :type Primitive%20Component%20Object%20Reference) (OtherBodyIndex :type Integer) (bFromSweep :type Boolean) (SweepResult :type Hit%20Result%20Structure%20%28by%20ref%29))
  (Utilities|Casting|CastToFirstPersonCharacter OtherActor)
  (bind _asgm_endless_fps2 (Utilities|Casting|CastToGM_EndlessFPS2 (Game|GetGameMode)))
  (Variables|/Game/Blueprint/Logic/GM_EndlessFPS2.GM_EndlessFPS2_C|SetDirection _asgm_endless_fps2 1)
  (Variables|/Game/Blueprint/Logic/GM_EndlessFPS2.GM_EndlessFPS2_C|SetIsTwoRoads _asgm_endless_fps2 false))

(event OnComponentBeginOverlap(RightBox)
  (params (OverlappedComponent :type Primitive%20Component%20Object%20Reference) (OtherActor :type Actor%20Object%20Reference) (OtherComp :type Primitive%20Component%20Object%20Reference) (OtherBodyIndex :type Integer) (bFromSweep :type Boolean) (SweepResult :type Hit%20Result%20Structure%20%28by%20ref%29))
  (Utilities|Casting|CastToFirstPersonCharacter OtherActor)
  (bind _asgm_endless_fps2 (Utilities|Casting|CastToGM_EndlessFPS2 (Game|GetGameMode)))
  (Variables|/Game/Blueprint/Logic/GM_EndlessFPS2.GM_EndlessFPS2_C|SetDirection _asgm_endless_fps2 2)
  (Variables|/Game/Blueprint/Logic/GM_EndlessFPS2.GM_EndlessFPS2_C|SetIsTwoRoads _asgm_endless_fps2 false))

(event EventBeginPlay
  (|CallParentFunction) ; This node is disabled and will not be called.\nDrag off pins to build functionality.
)

(event Collision|EventActorBeginOverlap
  (params (OtherActor :type Actor%20Object%20Reference))
  (|CallParentFunction OtherActor) ; This node is disabled and will not be called.\nDrag off pins to build functionality.
)

(event EventTick
  (params (DeltaSeconds :type Float%20%28single-precision%29))
  (|CallParentFunction DeltaSeconds) ; This node is disabled and will not be called.\nDrag off pins to build functionality.
)

(fn ConstructionScript
  (|CallParentFunction))