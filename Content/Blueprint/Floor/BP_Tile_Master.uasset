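; BP_Tile_Master is a floor tile actor, apparently a base for modular level pieces, that can populate itself with enemies.
; On BeginPlay, if SpawnEnemies is set, it gives each of three spawn points an independent coin-flip chance to spawn a BP_Enemy_AI.
; GetAttatchTransform exposes the world transforms of two attach points, AttatchPoint and Arrow.
; The DestroyTileTimer event destroys the tile after a short delay.
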(event Custom|DestroyTileTimer
  (Utilities|FlowControl|Delay 3.0)
  (Actor|DestroyActor))

(event EventBeginPlay
  (if (Variables|Default|GetSpawnEnemies)
    (if (== (Math|Random|RandomIntegerinRange 0 1) 0)
      (Game|SpawnActorfromClass "/Game/Blueprint/BP_Enemy_AI.BP_Enemy_AI_C" (Transformation|GetWorldTransform (Variables|Default|GetEnemySpawn1)) "Undefined" 0 0))
    (if (== (Math|Random|RandomIntegerinRange 0 1) 0)
      (Game|SpawnActorfromClass "/Game/Blueprint/BP_Enemy_AI.BP_Enemy_AI_C" (Transformation|GetWorldTransform (Variables|Default|GetEnemySpawn2)) "Undefined" 0 0))
    (if (== (Math|Random|RandomIntegerinRange 0 1) 0)
      (Game|SpawnActorfromClass "/Game/Blueprint/BP_Enemy_AI.BP_Enemy_AI_C" (Transformation|GetWorldTransform (Variables|Default|GetEnemySpawn3)) "Undefined" 0 0))))

(fn ConstructionScript)

(fn GetAttatchTransform
  (return (Transformation|GetWorldTransform (Variables|Default|GetAttatchPoint)) (Transformation|GetWorldTransform (Variables|Default|GetArrow))))