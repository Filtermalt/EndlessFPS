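; Game mode Blueprint that manages a chain of BP_Spawner actors and their sequential tile destruction.
; AddSpawner spawns a spawner at NextSpawnPoint and appends it to SpawnerArray.
; DestroyTilesCheck advances the index once the current spawner is invalid, then starts tile destruction on the next.
; BeginPlay is empty, leaving the initial spawning and looping timer that drives this check disconnected.
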(event EventBeginPlay)

(fn ConstructionScript)

(fn AddSpawner
  (bind _returnvalue (Game|SpawnActorfromClass "/Game/Blueprint/Floor/BP_Spawner.BP_Spawner_C" (Variables|Default|GetNextSpawnPoint) "Undefined" 0 0))
  (Utilities|Array|Add (Variables|Default|GetSpawnerArray) _returnvalue))

(fn DestroyTilesCheck
  (Utilities|IsValid (Utilities|Array|Get(acopy) (Variables|Default|GetSpawnerArray) (Variables|Default|Getindex))
    (:Is%20Not%20Valid
      (Variables|Default|Setindex (+ (Variables|Default|Getindex) 1))
      (Default|StartDestroyTiles (Utilities|Array|Get(acopy) (Variables|Default|GetSpawnerArray) (Variables|Default|Getindex))))))