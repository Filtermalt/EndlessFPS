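; Endless-floor segment spawner for the endless FPS game mode, building a run of tiles and later breaking it up.
; On BeginPlay it chains ten forward tiles by attach transforms, randomly appends a BP_Tile_None, and saves the next spawn point to the game mode.
; StartDestroyTiles shatters tiles in order on a looping timer, then requests another spawner from the game mode and destroys itself.
; Left and right turn branches are unwired.
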(event Custom|StartDestroyTiles
  (CallFunction|DestroyTiles)
  (Utilities|Time|SetTimerbyFunctionName 0 "DestroyTiles" (Variables|Default|GetDestroyTilesTimer) true))

(event EventBeginPlay
  (bind _asgm_endless_fps2 (Utilities|Casting|CastToGM_EndlessFPS2 (Game|GetGameMode)))
  (Variables|Default|SetGameMode _asgm_endless_fps2)
  (Variables|Default|SetAttatchPoint (Variables|/Game/Blueprint/Logic/GM_EndlessFPS2.GM_EndlessFPS2_C|GetNextSpawnPoint (Variables|Default|GetGameMode)))
  (for _index (range 0 9)
    (CallFunction|AddTile))
  (CallFunction|AddTileTurn)
  (Variables|/Game/Blueprint/Logic/GM_EndlessFPS2.GM_EndlessFPS2_C|SetNextSpawnPoint (Variables|Default|GetGameMode) (Variables|Default|GetAttatchPoint)))

(fn ConstructionScript)

(fn AddTile
  (bind _returnvalue (Game|SpawnActorfromClass "/Game/Blueprint/Floor/BP_Tile_Forward.BP_Tile_Forward_C" (Variables|Default|GetAttatchPoint) "Undefined" 0 0))
  (Utilities|Array|Add (Variables|Default|GetTilesArray) _returnvalue)
  (bind _attatchtransform (Default|GetAttatchTransform _returnvalue))
  (Variables|Default|SetAttatchPoint _attatchtransform))

(fn SetNewSpawnPoint
  (return (Variables|Default|GetAttatchPoint)))

(fn DestroyTiles
  (Utilities|IsValid (Utilities|Array|Get(acopy) (Variables|Default|GetTilesArray) (Variables|Default|GetIndex))
    (:Is%20Valid
      (bind _returnvalue (AddComponent|AddDestructibleComponent (Utilities|Array|Get(acopy) (Variables|Default|GetTilesArray) (Variables|Default|GetIndex)) false))
      (Class|DestructibleComponent|ApplyDamage _returnvalue 5e+01 (Transformation|GetWorldLocation (Variables|/Script/Engine.Actor|GetRootComponent (Utilities|Array|Get(acopy) (Variables|Default|GetTilesArray) (Variables|Default|GetIndex)))) (Transformation|GetWorldLocation (Variables|/Script/Engine.Actor|GetRootComponent (Utilities|Array|Get(acopy) (Variables|Default|GetTilesArray) (Variables|Default|GetIndex)))) 1e+02)
      (Development|SetHiddeninGame (Variables|/Game/Blueprint/Floor/BP_Tile_Master.BP_Tile_Master_C|GetStaticMesh (Utilities|Array|Get(acopy) (Variables|Default|GetTilesArray) (Variables|Default|GetIndex))) true false)
      (Collision|SetCollisionEnabled (Variables|/Game/Blueprint/Floor/BP_Tile_Master.BP_Tile_Master_C|GetStaticMesh (Utilities|Array|Get(acopy) (Variables|Default|GetTilesArray) (Variables|Default|GetIndex))) "NoCollision")
      (Default|DestroyTileTimer (Utilities|Array|Get(acopy) (Variables|Default|GetTilesArray) (Variables|Default|GetIndex)))
      (Variables|Default|SetIndex (+ (Variables|Default|GetIndex) 1)))
    (:Is%20Not%20Valid
      (Default|AddSpawner (Variables|Default|GetGameMode))
      (Actor|DestroyActor))))

(fn AddTileTurn
  (switch int (Math|Random|RandomIntegerinRange 0 2)
    (:0
      _)
    (:2
      _))
  (bind _returnvalue (Game|SpawnActorfromClass "/Game/Blueprint/Floor/BP_Tile_None.BP_Tile_None_C" (Variables|Default|GetAttatchPoint) "Undefined" 0 0))
  (Utilities|Array|Add (Variables|Default|GetTilesArray) _returnvalue)
  (bind _attatchtransform (Default|GetAttatchTransform _returnvalue))
  (Variables|Default|SetAttatchPoint _attatchtransform)
  (Variables|Default|SetNewVar_0 true))