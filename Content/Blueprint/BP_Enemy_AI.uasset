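; Enemy actor that takes damage, gets knocked by impulses and dies; despite the AI name, it holds no decision logic here.
; Construction gives the mesh a random dynamic material, and sight events swap materials while it is alive.
; AnyDamage feeds CalculateHealth, then either applies a PlayerLocation-scaled capsule impulse or calls Death.
; Death applies a stronger impulse, ignores Pawn collision and sets a dead material.
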(event Custom|SetEnemyInSightColor
  ;[1 1 1] Is Targeted?
  (if (not (Variables|Default|GetIsDead))
    (Rendering|Material|SetMaterial (Variables|Default|GetStaticMesh) 0 0)))

(event Custom|SetEnemyNotInSightColor
  ;[1 1 1] Is Targeted?
  (if (not (Variables|Default|GetIsDead))
    (Rendering|Material|SetMaterial (Variables|Default|GetStaticMesh) 0 "/Game/FirstPerson/Meshes/FirstPersonProjectileMaterial.FirstPersonProjectileMaterial")))

(event Custom|Death
  ;[1 1 1] Set Death
  (Development|PrintString "Dead")
  (Physics|AddImpulse (Variables|Collision|GetCapsuleComponent) (* (Variables|Default|GetPlayerLocation) 2e+05) "None" false)
  (Collision|SetCollisionResponsetoChannel (Variables|Collision|GetCapsuleComponent) "ECC_Pawn" "ECR_Ignore")
  (Variables|Default|SetIsDead true)
  (Rendering|Material|SetMaterial (Variables|Default|GetStaticMesh) 0 "/Game/Geometry/Meshes/CubeMaterial.CubeMaterial"))

(event Custom|CustomEvent_0
  (params (NewParam :type Float%20%28single-precision%29)))

(event EventAffectHealth
  (params (Delta :type Float%20%28single-precision%29)))

(event EventBeginPlay
  (Variables|Default|SetCurrentHealth (Variables|Default|GetMaxHealth)))

(event Game|Damage|EventAnyDamage
  (params (Damage :type Float%20%28single-precision%29) (DamageType :type Damage%20Type%20Object%20Reference) (InstigatedBy :type Controller%20Object%20Reference) (DamageCauser :type Actor%20Object%20Reference))
  ;[1 1 1] Set health
  (bind _isdead (CallFunction|CalculateHealth Damage))
  (if _isdead
    (CallFunction|Death)
    (else
      (Physics|AddImpulse (Variables|Collision|GetCapsuleComponent) (* (Variables|Default|GetPlayerLocation) 9e+04) "None" false))))

(fn ConstructionScript
  (bind _staticmesh (Variables|Default|GetStaticMesh))
  (bind _output_get (Variables|Default|SetTypeIndex (Math|Random|RandomIntegerinRange 0 1)))
  (bind _returnvalue (Rendering|Material|CreateDynamicMaterialInstance _staticmesh 0 (Utilities|Array|Get(acopy) (Variables|Default|GetMaterialArray) _output_get) "None" :!class /Script/Engine.PrimitiveComponent))
  (Rendering|Material|SetMaterial _staticmesh 0 _returnvalue))

(fn CalculateHealth
  (params (Delta :type Float%20%28single-precision%29))
  (bind _output_get (Variables|Default|SetCurrentHealth (- (Variables|Default|GetCurrentHealth) Delta)))
  (bind _output_get_2 (Variables|Default|SetIsDead (<= _output_get 0.0)))
  (return _output_get_2))